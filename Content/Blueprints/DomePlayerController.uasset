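; DomePlayerController is a player controller that switches input between aligned actors and can reset the view to its starting state.
; BeginPlay stores the controlled BP_TrackPawn with its location and the control rotation.
; Input_Two disables input on every AlignedActors entry, unpossessing within that loop, then enables input on the first entry.
; ResetView restores the saved location and rotation and repossesses the track pawn.
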(event `InputAction|Input_Two`
  (params (Key :type "Key Structure"))
  (:`Pressed`
    (`self.Disable Inputs`)
    (if (> (`KismetArrayLibrary.Array_Length` (`self.AlignedActors`)) 0)
      (`self.EnableInput` (`|GetArrayItem` (`self.AlignedActors`)) self))))

(event `self.ReceiveBeginPlay`
  ;[0 0.1339 1] Setup of initial values
  (bind _asbp_track_pawn (cast `/Game/Blueprints/BP_TrackPawn` (`self.K2_GetPawn`)))
  (bind _output_get (set `self.DefaultPawn` _asbp_track_pawn))
  (set `self.OriginPos` (`self.K2_GetActorLocation` _output_get))
  (set `self.OriginRot` (`self.GetControlRotation`)))

(event `InputAction|ResetView`
  (params (Key :type "Key Structure"))
  ;[0 1 0.997] Resetting the view with the initial values
  (:`Released`
    (`self.K2_SetActorLocation` (`self.DefaultPawn`) (`self.OriginPos`) false false)
    (`self.SetControlRotation` (`self.OriginRot`))
    (`self.Possess` (`self.DefaultPawn`))))

(event `InputAction|Input_One`
  (params (Key :type "Key Structure"))
  ;[0.02316 0.6432 1] Add Input one
)

(event `InputAction|Input_Two`
  (params (Key :type "Key Structure"))
  ;[0 1 0.4685] Add Input 2
)

(event `InputAction|Input_Three`
  (params (Key :type "Key Structure"))
  ;[1 0.4349 0] Add input 3
)

(fn `Disable Inputs`
  (for _array_element (`self.AlignedActors`)
    (`self.DisableInput` _array_element self)
    (`self.UnPossess`)))

(fn `UserConstructionScript`)